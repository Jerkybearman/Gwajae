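; BP_Rocket is a short-lived projectile actor that destroys itself on hitting anything not tagged Player.
; BeginPlay gives it a three-second lifespan.
; On overlap with a non-Player actor, it calls ApplyDamage with no target or amount wired, prints that actor's name, spawns the NS_Base effect at its mesh location, then destroys itself.
; The file contains no movement logic.
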(event `self.ReceiveBeginPlay`
  (`self.SetLifeSpan` 3.0))

(event `self.ReceiveActorBeginOverlap`
  (params (OtherActor :type "Actor Object Reference"))
  (if (not (`self.ActorHasTag` OtherActor "Player"))
    (`GameplayStatics.ApplyDamage` null)
    (`KismetSystemLibrary.PrintString` (`KismetSystemLibrary.GetDisplayName` OtherActor))
    (`NiagaraFunctionLibrary.SpawnSystemAtLocation` "/Game/NS_Base.NS_Base" (`SceneComponent.K2_GetComponentLocation` (`self.StaticMesh`)))
    (`self.K2_DestroyActor`)))

(fn `UserConstructionScript`)